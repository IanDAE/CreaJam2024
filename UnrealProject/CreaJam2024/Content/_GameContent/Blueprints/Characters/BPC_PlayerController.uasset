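; Player controller for a top-down character that creates the game HUD and handles aiming, attack and pause input.
; Mouse movement enables cursor aim, turning control rotation toward a Visibility trace hit each tick, while movement input disables it and faces the input direction.
; Attack input calls the character's Attack behind a DoOnce with a delayed reset as a cooldown, and pause input forwards to the game mode.
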(event Input|EnhancedActionEvents|EnhancedInputActionIA_PlayerMovement
  (params (ActionValue :type Vector%202D%20Structure) (ElapsedSeconds :type Float%20%28double-precision%29) (TriggeredSeconds :type Float%20%28double-precision%29) (InputAction :type Input%20Action%20Object%20Reference :default "/Game/_GameContent/Input/IA_PlayerMovement.IA_PlayerMovement"))
  (bind _returnvalue (Pawn|GetControlledPawn))
  (bind _returnvalue_2 (Transformation|GetActorLocation _returnvalue))
  (:Triggered
    (Variables|Default|SetUseMouseAim false)
    (Pawn|SetControlRotation (Math|Rotator|FindLookatRotation _returnvalue_2 (+ _returnvalue_2 (Math|Vector|MakeVector (.y ActionValue) (.x ActionValue) (.Z (Class|KismetMathLibrary|BreakVector3f _returnvalue_2))))))))

(event Input|EnhancedActionEvents|EnhancedInputActionIA_PlayerAttack
  (params (ActionValue :type Boolean) (ElapsedSeconds :type Float%20%28double-precision%29) (TriggeredSeconds :type Float%20%28double-precision%29) (InputAction :type Input%20Action%20Object%20Reference :default "/Game/_GameContent/Input/IA_PlayerAttack.IA_PlayerAttack"))
  (:Triggered
    (Utilities|FlowControl|DoOnce false :!label _label
      (:Completed
        (bind _asbp_top_down_character (Utilities|Casting|CastToBP_TopDownCharacter (Pawn|GetControlledPawn)))
        (Default|Attack _asbp_top_down_character)
        (Utilities|FlowControl|Delay 0.7)
        (goto _label Reset)))))

(event Input|EnhancedActionEvents|EnhancedInputActionIA_PauseGame
  (params (ActionValue :type Boolean) (ElapsedSeconds :type Float%20%28double-precision%29) (TriggeredSeconds :type Float%20%28double-precision%29) (InputAction :type Input%20Action%20Object%20Reference :default "/Game/_GameContent/Input/IA_PauseGame.IA_PauseGame"))
  (:Triggered
    (bind _asbp_top_down_game_mode (Utilities|Casting|CastToBP_TopDownGameMode (Game|GetGameMode)))
    (Default|PauseGame _asbp_top_down_game_mode)))

(event EventBeginPlay
  (bind _returnvalue (PlayerController|LocalPlayerSubsystems|GetEnhancedInputLocalPlayerSubsystem))
  (Variables|Default|SetbShowMouseCursor true)
  (bind _returnvalue_2 (UserInterface|CreateWidget "/Game/_GameContent/Blueprints/UI/BPW_GameHud.BPW_GameHud_C"))
  (bind _output_get (Variables|Default|SetHUD _returnvalue_2))
  (UserInterface|Viewport|AddtoViewport _output_get 0)
  (Utilities|IsValid _returnvalue
    (:Is%20Valid
      (Input|AddMappingContext _returnvalue "/Game/_GameContent/Input/IMC_Player.IMC_Player" 0 "(bIgnoreAllPressedKeysUntilRelease=True,bForceImmediately=False)"))))

(event EventTick
  (params (DeltaSeconds :type Float%20%28single-precision%29))
  (bind _returnvalue (Pawn|GetControlledPawn))
  (bind (_hitresult _returnvalue_2) (Game|Player|GetHitResultUnderCursorbyChannel "TraceTypeQuery1" true))
  (bind _location (Collision|BreakHitResult _hitresult))
  (bind _returnvalue_3 (Transformation|GetActorLocation _returnvalue))
  (if (Variables|Default|GetUseMouseAim)
    ;[1 1 1] Rotate towards the mouse
    (if _returnvalue_2
      (if (> (Math|Vector|Distance(Vector) _returnvalue_3 _location) 5e+01)
        (Pawn|SetControlRotation (Math|Rotator|FindLookatRotation _returnvalue_3 _location))
        (Variables|Default|SetMouseLocation (- _location (Class|PlayerController|GetFocalLocation)))))))

(event Input|MouseEvents|Mouse2D
  (params (AxisValue :type Vector :default "0, 0, 0"))
  ;[1 1 1] Detect mouse movement
  (if (> (Class|KismetMathLibrary|VSizeXYSquared AxisValue) 0.0)
    (Variables|Default|SetUseMouseAim true)))

(fn ConstructionScript)