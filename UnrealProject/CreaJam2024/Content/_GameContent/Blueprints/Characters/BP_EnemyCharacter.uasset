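; BP_EnemyCharacter is an enemy character that senses the player's pawn, turns to face it, and destroys itself when health runs out.
; While enabled, Tick computes 2D distance and view angle to the player, then derives visible, in-attack-range and looking-at flags by threshold, without line traces.
; Those flags drive a smoothed turn toward the player or a movement stop.
; An AIMoveTo chase node exists but is unconnected.
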(event EventBeginPlay)

(event Collision|EventActorBeginOverlap
  (params (OtherActor :type Actor%20Object%20Reference)))

(event EventTick
  (params (DeltaSeconds :type Float%20%28single-precision%29))
  (bind _returnvalue (Transformation|GetActorLocation))
  (bind _returnvalue_2 (Game|GetPlayerController 0))
  (bind _returnvalue_3 (Pawn|GetControlledPawn _returnvalue_2))
  (bind _returnvalue_4 (Transformation|GetActorLocation _returnvalue_3))
  (if (Variables|Default|GetIsEnabled)
    (Utilities|FlowControl|Sequence
      (:then_0
        (if (<= (Variables|Default|GetHealth) 0.0)
          (Actor|DestroyActor)))
      (:then_1
        ;[1 1 1] Calculate distance to the player
        (Variables|Default|SetDistanceFromPlayer (Math|Vector|Distance2D(Vector) _returnvalue_4 _returnvalue))
        (Variables|Default|SetViewAngleToPlayer (Class|KismetMathLibrary|DegAcos (Math|Vector|DotProduct (Math|Vector|Normalize (Transformation|GetActorForwardVector)) (Math|Vector|Normalize (- _returnvalue_4 _returnvalue))))))
      (:then_2
        (Variables|Default|SetIsPlayerVisible (<= (Variables|Default|GetDistanceFromPlayer) (Variables|Default|GetVisibilityRange)))
        (Variables|Default|SetIsInAttackRange (<= (Variables|Default|GetDistanceFromPlayer) (Variables|Default|GetAttackRange)))
        (Variables|Default|SetIsLookingAtPlayer (<= (Variables|Default|GetViewAngleToPlayer) (Variables|Default|GetViewRange))))
      (:then_3
        (if (Variables|Default|GetIsPlayerVisible)
          (if (Variables|Default|GetIsLookingAtPlayer)
            (if (Variables|Default|GetIsInAttackRange)
              (Class|NavMovementComponent|StopActiveMovement (Variables|Character|GetCharacterMovement)))
            (else
              (Transformation|SetActorRotation (Math|Rotator|Lerp(Rotator) (Transformation|GetActorRotation) (Math|Rotator|FindLookatRotation (Transformation|GetActorLocation) (Transformation|GetActorLocation (Pawn|GetControlledPawn (Game|GetPlayerController 0)))) (* (Utilities|Time|GetWorldDeltaSeconds) 1e+01) true))))
          (else
            (Class|NavMovementComponent|StopActiveMovement (Variables|Character|GetCharacterMovement))))))))

(fn ConstructionScript)