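; BP_1FloorPrefabZ is a floor tile prefab that varies its look when play begins.
; BeginPlay gives Tile01 a random mesh from TileArray, then RandomSeed slightly shrinks it and returns a rotation with small random tilt and yaw.
; The intended quarter-turn yaw never applies because the location-based seed always truncates to zero, so yaw is only jitter around world zero.
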(event EventBeginPlay
  (bind _tile01 (Variables|Default|Gettile01))
  (Components|StaticMesh|SetStaticMesh (Variables|Default|Gettile01) (Utilities|Array|Get(acopy) (Variables|Default|GetTileArray) (Math|Random|RandomIntegerinRange 0 2)))
  (bind _outrotator (CallFunction|RandomSeed _tile01))
  (Transformation|SetWorldRotation _tile01 _outrotator false false))

(fn ConstructionScript)

(fn RandomSeed
  (params (Target :type Scene%20Component%20Object%20Reference))
  (bind _returnvalue (Transformation|GetWorldRotation Target))
  (bind _returnvalue_2 (Transformation|GetWorldLocation Target))
  (bind _output_get (Variables|Default|SetSeed (Math|Float|Truncate (Math|Float|%(Float) (* (.x _returnvalue_2) (.y _returnvalue_2)) 1.0))))
  (Transformation|SetWorldScale3D Target (* (Transformation|GetWorldScale Target) (Math|Random|RandomFloatinRange 0.97 1.0)))
  (return (Math|Rotator|MakeRotator (+ (Math|Random|RandomFloatinRange -3.0 3.0) (.roll _returnvalue)) (+ (.pitch _returnvalue) (Math|Random|RandomFloatinRange -3.0 3.0)) (+ (* 9e+01 (* _output_get (Math|Random|RandomIntegerinRange 0 4))) (Math|Random|RandomFloatinRange -3.0 3.0)))))