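; Floor prefab of four tiles that aims to vary its look at runtime.
; On BeginPlay each tile gets a random mesh from the first three TileArray entries, then a world rotation from the RandomSeed function.
; RandomSeed keeps roll and yaw and sets pitch to a near-90-degree random step times a location-derived seed.
; That seed truncates a modulo-1 value, so it evaluates to zero and flattens the pitch.
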(event EventBeginPlay
  (bind _tile02 (Variables|Default|Gettile02))
  (bind _tile04 (Variables|Default|Gettile04))
  (bind _tile03 (Variables|Default|Gettile03))
  (bind _tile01 (Variables|Default|Gettile01))
  (Components|StaticMesh|SetStaticMesh (Variables|Default|Gettile01) (Utilities|Array|Get(acopy) (Variables|Default|GetTileArray) (Math|Random|RandomIntegerinRange 0 2)))
  (Components|StaticMesh|SetStaticMesh (Variables|Default|Gettile03) (Utilities|Array|Get(acopy) (Variables|Default|GetTileArray) (Math|Random|RandomIntegerinRange 0 2)))
  (Components|StaticMesh|SetStaticMesh (Variables|Default|Gettile02) (Utilities|Array|Get(acopy) (Variables|Default|GetTileArray) (Math|Random|RandomIntegerinRange 0 2)))
  (Components|StaticMesh|SetStaticMesh (Variables|Default|Gettile04) (Utilities|Array|Get(acopy) (Variables|Default|GetTileArray) (Math|Random|RandomIntegerinRange 0 2)))
  (bind _outrotator (CallFunction|RandomSeed (Variables|Default|GetSeed) _tile02))
  (Transformation|SetWorldRotation _tile02 _outrotator false false)
  (bind _outrotator_2 (CallFunction|RandomSeed (Variables|Default|GetSeed) _tile03))
  (Transformation|SetWorldRotation _tile03 _outrotator_2 false false)
  (bind _outrotator_3 (CallFunction|RandomSeed (Variables|Default|GetSeed) _tile01))
  (Transformation|SetWorldRotation _tile01 _outrotator_3 false false)
  (bind _outrotator_4 (CallFunction|RandomSeed (Variables|Default|GetSeed) _tile04))
  (Transformation|SetWorldRotation _tile04 _outrotator_4 false false))

(event Collision|EventActorBeginOverlap
  (params (OtherActor :type Actor%20Object%20Reference)))

(event EventTick
  (params (DeltaSeconds :type Float%20%28single-precision%29)))

(fn ConstructionScript)

(fn RandomSeed
  (params (seed :type Integer) (Target :type Scene%20Component%20Object%20Reference))
  (bind _returnvalue (Transformation|GetWorldRotation Target))
  (bind _returnvalue_2 (Transformation|GetWorldLocation Target))
  (bind _output_get (Variables|Default|SetSeed (Math|Float|Truncate (Math|Float|%(Float) (* (.x _returnvalue_2) (.y _returnvalue_2)) 1.0))))
  (return (Math|Rotator|MakeRotator (.roll _returnvalue) (* (Math|Random|RandomFloatinRange 86.0 93.0) (* _output_get (Math|Random|RandomIntegerinRange 0 4))) (.yaw _returnvalue))))