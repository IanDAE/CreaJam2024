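; BP_Braiser is a brazier prefab that flickers its SpotLightFront2 spotlight, apparently to mimic firelight.
; Every Tick it calls LightVariations, which nudges outer cone angle and intensity by random offsets scaled through a Lerp alpha, with intensity using double the smoothing factor.
; Each step builds on the current value, giving a random walk that is clamped to fixed angle and brightness ranges.
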(event EventBeginPlay)

(event EventTick
  (params (DeltaSeconds :type Float%20%28single-precision%29))
  (CallFunction|LightVariations (Variables|Default|GetSpotLightFront2) 5e+02 2e+01 0.1))

(fn ConstructionScript)

(fn LightVariations
  (params (InLight :type Spot%20Light%20Component%20Object%20Reference) (IntensityVar :type Float%20%28double-precision%29) (AngleVar :type Float%20%28double-precision%29) (VarSmoothness :type Float%20%28double-precision%29))
  (bind _intensity (Variables|/Script/Engine.LightComponentBase|GetIntensity InLight))
  (bind _outerconeangle (Variables|/Script/Engine.SpotLightComponent|GetOuterConeAngle InLight))
  (Rendering|Lighting|SetOuterConeAngle InLight (Math|Float|Clamp(Float) (Math|Float|Lerp _outerconeangle (+ _outerconeangle (Math|Random|RandomFloatinRange (* AngleVar -1.0) AngleVar)) VarSmoothness) 55.0 1.2e+02))
  (Rendering|Components|Light|SetIntensity InLight (Math|Float|Clamp(Float) (Math|Float|Lerp _intensity (+ _intensity (Math|Random|RandomFloatinRange (* IntensityVar -1.0) IntensityVar)) (* VarSmoothness 2.0)) 6.5e+02 3e+03)))