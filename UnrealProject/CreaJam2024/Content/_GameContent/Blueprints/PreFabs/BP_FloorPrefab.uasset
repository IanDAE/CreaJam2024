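; BP_FloorPrefab is a floor prefab of four tiles that randomizes its look on BeginPlay.
; Each tile gets a random mesh from the first three TileArray entries, then a world yaw from RandomSeed.
; RandomSeed multiplies random near-right-angle steps by a location-derived seed.
; That seed truncates a modulo-1 result to zero, so the yaw always evaluates to zero.
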(event EventBeginPlay
  (bind _tile02 (Variables|Default|Gettile02))
  (bind _tile04 (Variables|Default|Gettile04))
  (bind _tile03 (Variables|Default|Gettile03))
  (bind _tile01 (Variables|Default|Gettile01))
  (Components|StaticMesh|SetStaticMesh (Variables|Default|Gettile01) (Utilities|Array|Get(acopy) (Variables|Default|GetTileArray) (Math|Random|RandomIntegerinRange 0 2)))
  (Components|StaticMesh|SetStaticMesh (Variables|Default|Gettile03) (Utilities|Array|Get(acopy) (Variables|Default|GetTileArray) (Math|Random|RandomIntegerinRange 0 2)))
  (Components|StaticMesh|SetStaticMesh (Variables|Default|Gettile02) (Utilities|Array|Get(acopy) (Variables|Default|GetTileArray) (Math|Random|RandomIntegerinRange 0 2)))
  (Components|StaticMesh|SetStaticMesh (Variables|Default|Gettile04) (Utilities|Array|Get(acopy) (Variables|Default|GetTileArray) (Math|Random|RandomIntegerinRange 0 2)))
  (bind _outyaw (CallFunction|RandomSeed (Variables|Default|GetSeed) _tile02))
  (Transformation|SetWorldRotation _tile02 (Math|Rotator|MakeRotator 0.0 0.0 _outyaw) false false)
  (bind _outyaw_2 (CallFunction|RandomSeed (Variables|Default|GetSeed) _tile03))
  (Transformation|SetWorldRotation _tile03 (Math|Rotator|MakeRotator 0.0 0.0 _outyaw_2) false false)
  (bind _outyaw_3 (CallFunction|RandomSeed (Variables|Default|GetSeed) _tile01))
  (Transformation|SetWorldRotation _tile01 (Math|Rotator|MakeRotator 0.0 0.0 _outyaw_3) false false)
  (bind _outyaw_4 (CallFunction|RandomSeed (Variables|Default|GetSeed) _tile04))
  (Transformation|SetWorldRotation _tile04 (Math|Rotator|MakeRotator 0.0 0.0 _outyaw_4) false false))

(event Collision|EventActorBeginOverlap
  (params (OtherActor :type Actor%20Object%20Reference)))

(event EventTick
  (params (DeltaSeconds :type Float%20%28single-precision%29)))

(fn ConstructionScript)

(fn RandomSeed
  (params (seed :type Integer) (Target :type Scene%20Component%20Object%20Reference))
  (bind _returnvalue (Transformation|GetWorldLocation Target))
  (bind _output_get (Variables|Default|SetSeed (Math|Float|Truncate (Math|Float|%(Float) (* (.x _returnvalue) (.y _returnvalue)) 1.0))))
  (return (* (Math|Random|RandomFloatinRange 86.0 93.0) (* _output_get (Math|Random|RandomIntegerinRange 0 4)))))