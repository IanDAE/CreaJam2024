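; Pillar prefab with four torches, faked by eight front and back spotlights that flicker.
; On BeginPlay, RandomSeed slightly shrinks the pillar and jitters its rotation; the position-derived seed truncates to zero, so the intended 90-degree yaw steps drop out.
; Every Tick, LightVariations random-walks each spotlight's cone angle, intensity and color temperature with a lerped, clamped offset.
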(event EventBeginPlay
  (bind _pillar (Variables|Default|GetPillar))
  (bind _outrotator (CallFunction|RandomSeed _pillar))
  (Transformation|SetWorldRotation _pillar _outrotator false false))

(event EventTick
  (params (DeltaSeconds :type Float%20%28single-precision%29))
  (CallFunction|LightVariations (Variables|Default|GetSpotLightBack2) 6e+02 25.0 5e+01 0.1)
  (CallFunction|LightVariations (Variables|Default|GetSpotLightFront2) 6e+02 25.0 5e+01 0.1)
  (CallFunction|LightVariations (Variables|Default|GetSpotLightBack1) 6e+02 25.0 5e+01 0.1)
  (CallFunction|LightVariations (Variables|Default|GetSpotLightFront1) 6e+02 25.0 5e+01 0.1)
  (CallFunction|LightVariations (Variables|Default|GetSpotLightBack) 6e+02 25.0 5e+01 0.1)
  (CallFunction|LightVariations (Variables|Default|GetSpotLightFront) 6e+02 25.0 5e+01 0.1)
  (CallFunction|LightVariations (Variables|Default|GetSpotLightFront3) 6e+02 25.0 5e+01 0.1)
  (CallFunction|LightVariations (Variables|Default|GetSpotLightBack3) 6e+02 25.0 5e+01 0.1))

(fn ConstructionScript)

(fn RandomSeed
  (params (Target :type Scene%20Component%20Object%20Reference))
  (bind _returnvalue (Transformation|GetWorldRotation Target))
  (bind _returnvalue_2 (Transformation|GetWorldLocation Target))
  (bind _output_get (Variables|Default|SetSeed (Math|Float|Truncate (Math|Float|%(Float) (* (.x _returnvalue_2) (.y _returnvalue_2)) 1.0))))
  (Transformation|SetWorldScale3D Target (* (Transformation|GetWorldScale Target) (Math|Random|RandomFloatinRange 0.97 1.0)))
  (return (Math|Rotator|MakeRotator (+ (Math|Random|RandomFloatinRange -3.0 3.0) (.roll _returnvalue)) (+ (.pitch _returnvalue) (Math|Random|RandomFloatinRange -3.0 3.0)) (+ (* 9e+01 (* _output_get (Math|Random|RandomIntegerinRange 0 4))) (Math|Random|RandomFloatinRange -3.0 3.0)))))

(fn LightVariations
  (params (InLight :type Spot%20Light%20Component%20Object%20Reference) (IntensityVar :type Float%20%28double-precision%29) (AngleVar :type Float%20%28double-precision%29) (TempVar :type Float%20%28double-precision%29) (VarSmoothness :type Float%20%28double-precision%29))
  (bind _temperature (Variables|/Script/Engine.LightComponent|GetTemperature InLight))
  (bind _intensity (Variables|/Script/Engine.LightComponentBase|GetIntensity InLight))
  (bind _outerconeangle (Variables|/Script/Engine.SpotLightComponent|GetOuterConeAngle InLight))
  (Rendering|Lighting|SetOuterConeAngle InLight (Math|Float|Clamp(Float) (Math|Float|Lerp _outerconeangle (+ _outerconeangle (Math|Random|RandomFloatinRange (* AngleVar -1.0) AngleVar)) VarSmoothness) 55.0 1.2e+02))
  (Rendering|Components|Light|SetIntensity InLight (Math|Float|Clamp(Float) (Math|Float|Lerp _intensity (+ _intensity (Math|Random|RandomFloatinRange (* IntensityVar -1.0) IntensityVar)) (* VarSmoothness 2.0)) 6.5e+02 3e+03))
  (Class|LightComponent|SetTemperature InLight (Math|Float|Clamp(Float) (Math|Float|Lerp _temperature (+ _temperature (Math|Random|RandomFloatinRange (* TempVar -1.0) TempVar)) VarSmoothness) 1.25e+03 1.7e+03)))