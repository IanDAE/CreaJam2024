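; Checkpoint prop that registers room data with the top-down game mode when triggered.
; At BeginPlay it caches the starting transforms of the valid actors in its RoomEnemies list.
; Its Triggered event passes the new-room flag, start and max time, its own transform as player start, and those cached transforms to BP_TopDownGameMode through SetRoomData.
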(event EventBeginPlay
  (|CallParentFunction)
  (for _array_element (Variables|Default|GetRoomEnemies)
    (Utilities|IsValid _array_element
      (:Is%20Valid
        (Utilities|Array|Add (Variables|Default|GetEnemyPositions) (Transformation|GetActorTransform _array_element))))))

(event Collision|EventActorBeginOverlap
  (params (OtherActor :type Actor%20Object%20Reference))
  (|CallParentFunction OtherActor) ; This node is disabled and will not be called.\nDrag off pins to build functionality.
)

(event EventTick
  (params (DeltaSeconds :type Float%20%28single-precision%29))
  (|CallParentFunction DeltaSeconds) ; This node is disabled and will not be called.\nDrag off pins to build functionality.
)

(event EventTriggered
  (params (PlayerCharacter :type BP%20Top%20Down%20Character%20Object%20Reference))
  (bind _asbp_top_down_game_mode (Utilities|Casting|CastToBP_TopDownGameMode (Game|GetGameMode)))
  (Default|SetRoomData _asbp_top_down_game_mode (Variables|Default|GetIsNewRoom) (Variables|Default|GetStartTime) (Variables|Default|GetMaxTime) (Transformation|GetActorTransform) (Variables|Default|GetEnemyPositions)))

(fn ConstructionScript
  (|CallParentFunction))