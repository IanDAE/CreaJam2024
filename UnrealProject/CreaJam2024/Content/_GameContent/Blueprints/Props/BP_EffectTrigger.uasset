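; BP_EffectTrigger is a prop that applies a timed speed effect to the player character passed to its PickedUp event.
; The event sets the character's SpeedMultiplier to EffectSpeedMultiplier, then waits for EffectTime.
; It then restores the multiplier to 1.0 only if the character is still valid and the value is unchanged, leaving a different active multiplier intact.
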(event EventBeginPlay
  (|CallParentFunction) ; This node is disabled and will not be called.\nDrag off pins to build functionality.
)

(event Collision|EventActorBeginOverlap
  (params (OtherActor :type Actor%20Object%20Reference))
  (|CallParentFunction OtherActor) ; This node is disabled and will not be called.\nDrag off pins to build functionality.
)

(event EventTick
  (params (DeltaSeconds :type Float%20%28single-precision%29))
  (|CallParentFunction DeltaSeconds) ; This node is disabled and will not be called.\nDrag off pins to build functionality.
)

(event EventPickedUp
  (params (PlayerCharacter :type BP%20Top%20Down%20Character%20Object%20Reference))
  (Variables|/Game/TopDown/Blueprints/BP_TopDownCharacter.BP_TopDownCharacter_C|SetSpeedMultiplier PlayerCharacter (Variables|Default|GetEffectSpeedMultiplier))
  (Utilities|FlowControl|Delay (Variables|Default|GetEffectTime))
  (Utilities|IsValid PlayerCharacter
    (:Is%20Valid
      (if (== (Variables|/Game/TopDown/Blueprints/BP_TopDownCharacter.BP_TopDownCharacter_C|GetSpeedMultiplier PlayerCharacter) (Variables|Default|GetEffectSpeedMultiplier))
        (Variables|/Game/TopDown/Blueprints/BP_TopDownCharacter.BP_TopDownCharacter_C|SetSpeedMultiplier PlayerCharacter 1.0)))))

(fn ConstructionScript
  (|CallParentFunction))