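; Slime effect trigger prop that randomizes the look of its Plane mesh when play begins.
; After calling the parent BeginPlay, it picks one of three meshes from an array, sets a random yaw with zero pitch and roll, and multiplies the world scale by a random factor.
; The file adds no overlap or effect logic of its own.
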(event EventBeginPlay
  (bind _plane (Variables|Default|GetPlane))
  (|CallParentFunction)
  (Components|StaticMesh|SetStaticMesh (Variables|Default|GetPlane) (Utilities|Array|Get(acopy) (Variables|Default|Getstatic%20mesh) (Math|Random|RandomIntegerinRange 0 2)))
  (Transformation|SetWorldRotation _plane (Math|Rotator|MakeRotator 0.0 0.0 (Math|Random|RandomFloatinRange 0.0 3.6e+02)) false false)
  (Transformation|SetWorldScale3D _plane (* (Math|Random|RandomFloatinRange 1.0 2.0) (Transformation|GetWorldScale _plane))))

(event Collision|EventActorBeginOverlap
  (params (OtherActor :type Actor%20Object%20Reference))
  (|CallParentFunction OtherActor) ; This node is disabled and will not be called.\nDrag off pins to build functionality.
)

(event EventTick
  (params (DeltaSeconds :type Float%20%28single-precision%29))
  (|CallParentFunction DeltaSeconds) ; This node is disabled and will not be called.\nDrag off pins to build functionality.
)

(fn ConstructionScript
  (|CallParentFunction))