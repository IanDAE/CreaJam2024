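; A speed variant of an effect trigger prop that marks itself with the speed trap mesh and plays a speed power-up sound.
; On BeginPlay it runs the parent logic, then sets its Plane component to the speed trap mesh.
; When a top-down character overlaps its Box, it plays the sound at the box's location.
; The graph itself applies no speed change.
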(event OnComponentBeginOverlap(Box)
  (params (OverlappedComponent :type Primitive%20Component%20Object%20Reference) (OtherActor :type Actor%20Object%20Reference) (OtherComp :type Primitive%20Component%20Object%20Reference) (OtherBodyIndex :type Integer) (bFromSweep :type Boolean) (SweepResult :type Hit%20Result%20Structure%20%28by%20ref%29))
  (Utilities|Casting|CastToBP_TopDownCharacter OtherActor)
  (Audio|PlaySoundatLocation "/Game/_GameContent/Audio/Effects/Sound_Cues/SC_SpeedPW.SC_SpeedPW" (Transformation|GetWorldLocation (Variables|Default|GetBox)) "0, 0, 0" 1.0 1.0 0.0 0 0 0 0))

(event EventBeginPlay
  (|CallParentFunction)
  (Components|StaticMesh|SetStaticMesh (Variables|Default|GetPlane) "/Game/_GameContent/Meshes/Props/SM_TrapSpeed.SM_TrapSpeed"))

(event Collision|EventActorBeginOverlap
  (params (OtherActor :type Actor%20Object%20Reference))
  (|CallParentFunction OtherActor) ; This node is disabled and will not be called.\nDrag off pins to build functionality.
)

(event EventTick
  (params (DeltaSeconds :type Float%20%28single-precision%29))
  (|CallParentFunction DeltaSeconds) ; This node is disabled and will not be called.\nDrag off pins to build functionality.
)

(fn ConstructionScript
  (|CallParentFunction))