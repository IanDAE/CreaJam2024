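; A prop trap that repeatedly fires projectiles, with an arrow trap mesh and sound.
; BeginPlay starts a looping timer using a configurable fire delay and initial start offset.
; Each timer tick spawns the configured ProjectileType at the FireSocket transform and plays the arrow trap sound at the trap head mesh's location.
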(event Custom|FireProjectile
  (Game|SpawnActorfromClass (Variables|Default|GetProjectileType) (Transformation|GetWorldTransform (Variables|Default|GetFireSocket)) "Undefined" "MultiplyWithRoot" 0 0)
  (Audio|PlaySoundatLocation "/Game/_GameContent/Audio/Effects/Sound_Cues/SC_Trap_Arrow.SC_Trap_Arrow" (Transformation|GetWorldLocation (Variables|Default|GetSM_TrapArrow_SM_SM_TrapArrow_head)) "0, 0, 0" 1.0 1.0 0.0 0 0 0 0))

(event EventBeginPlay
  (Utilities|Time|SetTimerbyEvent (delegate Custom|FireProjectile) (Variables|Default|GetFireDelayTime) true (Variables|Default|GetStartOffsetTime)))

(event Collision|EventActorBeginOverlap
  (params (OtherActor :type Actor%20Object%20Reference)))

(event EventTick
  (params (DeltaSeconds :type Float%20%28single-precision%29)))

(fn ConstructionScript)