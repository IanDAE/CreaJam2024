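; BP_Spikes is a spike prop whose Cone component rises and lowers on a repeating timed cycle.
; Tick accumulates time and steps a four-state mode (Down, Moving Up, Up, Moving Down), carrying leftover time into each next phase.
; The mode then selects the Cone's relative height, interpolating linearly while moving.
; StartOffsetTime seeds the timer so instances can be staggered, and no overlap or damage logic is active here.
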(event EventBeginPlay
  (|CallParentFunction)
  (Variables|Default|SetTotalPassedTime (Variables|Default|GetStartOffsetTime)))

(event Collision|EventActorBeginOverlap
  (params (OtherActor :type Actor%20Object%20Reference))
  (|CallParentFunction OtherActor) ; This node is disabled and will not be called.\nDrag off pins to build functionality.
)

(event EventTick
  (params (DeltaSeconds :type Float%20%28single-precision%29))
  (bind _cone (Variables|Default|GetCone))
  (bind _relativelocation (Variables|/Script/Engine.SceneComponent|GetRelativeLocation _cone))
  (|CallParentFunction DeltaSeconds)
  (Variables|Default|SetTotalPassedTime (+ DeltaSeconds (Variables|Default|GetTotalPassedTime)))
  (Utilities|FlowControl|Sequence
    (:then_0
      (switch Utilities|FlowControl|Switch|SwitchonE_SpikeModes (Variables|Default|GetCurrentSpikeMode)
        (:NewEnumerator0
          (if (> (Variables|Default|GetTotalPassedTime) (Variables|Default|GetSpikeDownTime))
            (Variables|Default|SetTotalPassedTime (- (Variables|Default|GetTotalPassedTime) (Variables|Default|GetSpikeDownTime)))
            (Variables|Default|SetCurrentSpikeMode "NewEnumerator1")))
        (:NewEnumerator1
          (if (> (Variables|Default|GetTotalPassedTime) (Variables|Default|GetSpikeMovingTime))
            (Variables|Default|SetTotalPassedTime (- (Variables|Default|GetTotalPassedTime) (Variables|Default|GetSpikeMovingTime)))
            (Variables|Default|SetCurrentSpikeMode "NewEnumerator2")))
        (:NewEnumerator2
          (if (> (Variables|Default|GetTotalPassedTime) (Variables|Default|GetSpikeUpTime))
            (Variables|Default|SetTotalPassedTime (- (Variables|Default|GetTotalPassedTime) (Variables|Default|GetSpikeUpTime)))
            (Variables|Default|SetCurrentSpikeMode "NewEnumerator3")))
        (:NewEnumerator3
          (if (> (Variables|Default|GetTotalPassedTime) (Variables|Default|GetSpikeMovingTime))
            (Variables|Default|SetTotalPassedTime (- (Variables|Default|GetTotalPassedTime) (Variables|Default|GetSpikeMovingTime)))
            (Variables|Default|SetCurrentSpikeMode "NewEnumerator0")))))
    (:then_1
      (Transformation|SetRelativeLocation _cone (Math|Vector|MakeVector (.x _relativelocation) (.y _relativelocation) (Utilities|Select :Index (Variables|Default|GetCurrentSpikeMode) :NewEnumerator0 -5e+01 :NewEnumerator1 (- (* (- 1.0 (/ (Variables|Default|GetTotalPassedTime) (Variables|Default|GetSpikeMovingTime))) -4e+01) 1e+01) :NewEnumerator2 -1e+01 :NewEnumerator3 (- (* (/ (Variables|Default|GetTotalPassedTime) (Variables|Default|GetSpikeMovingTime)) -4e+01) 1e+01))) false false))))

(fn ConstructionScript
  (|CallParentFunction))