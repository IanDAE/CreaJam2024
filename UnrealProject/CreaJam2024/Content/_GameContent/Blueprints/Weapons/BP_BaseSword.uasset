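; Base sword weapon that damages and knocks back enemies it touches during an attack.
; An EnableCollision event sets the IsAttacking flag, which gates the Box component's overlap handler.
; On overlap with a BP_EnemyCharacter, it subtracts Damage directly from Health and calls the enemy's Knockback with Knockbackforce.
; Disconnected leftover nodes hold earlier physics force and impulse knockback attempts that never run.
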(event OnComponentBeginOverlap(Box)
  (params (OverlappedComponent :type Primitive%20Component%20Object%20Reference) (OtherActor :type Actor%20Object%20Reference) (OtherComp :type Primitive%20Component%20Object%20Reference) (OtherBodyIndex :type Integer) (bFromSweep :type Boolean) (SweepResult :type Hit%20Result%20Structure%20%28by%20ref%29))
  (if (Variables|Default|GetIsAttacking)
    (bind _asbp_enemy_character (Utilities|Casting|CastToBP_EnemyCharacter OtherActor))
    (Variables|/Game/_GameContent/Blueprints/Characters/BP_EnemyCharacter.BP_EnemyCharacter_C|SetHealth _asbp_enemy_character (- (Variables|/Game/_GameContent/Blueprints/Characters/BP_EnemyCharacter.BP_EnemyCharacter_C|GetHealth _asbp_enemy_character) (Variables|Default|GetDamage)))
    (Default|Knockback _asbp_enemy_character (Variables|Default|GetKnockbackforce))))

(event Custom|EnableCollision
  (params (IsTrue :type Boolean))
  (Variables|Default|SetIsAttacking IsTrue))

(event EventBeginPlay)

(event Collision|EventActorBeginOverlap
  (params (OtherActor :type Actor%20Object%20Reference)))

(event EventTick
  (params (DeltaSeconds :type Float%20%28single-precision%29)))

(fn ConstructionScript)